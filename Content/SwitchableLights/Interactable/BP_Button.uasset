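; BP_Button is an interactable switch actor, in the SwitchableLights folder, that toggles an on/off state.
; Its sphere collision registers it as the third-person character's ClosestButton on overlap and clears that reference when the overlap ends.
; ToggleButton flips IsOn and broadcasts the new state through the EDSwitch event dispatcher, so listeners can react without the button referencing them.
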(event OnComponentBeginOverlap(SphereCollision)
  (params (OverlappedComponent :type Primitive%20Component%20Object%20Reference) (OtherActor :type Actor%20Object%20Reference) (OtherComp :type Primitive%20Component%20Object%20Reference) (OtherBodyIndex :type Integer) (bFromSweep :type Boolean) (SweepResult :type Hit%20Result%20Structure%20%28by%20ref%29))
  (bind _asbp_third_person_character (Utilities|Casting|CastToBP_ThirdPersonCharacter OtherActor))
  (Variables|/Game/ThirdPerson/Blueprints/BP_ThirdPersonCharacter.BP_ThirdPersonCharacter_C|SetClosestButton _asbp_third_person_character self))

(event OnComponentEndOverlap(SphereCollision)
  (params (OverlappedComponent :type Primitive%20Component%20Object%20Reference) (OtherActor :type Actor%20Object%20Reference) (OtherComp :type Primitive%20Component%20Object%20Reference) (OtherBodyIndex :type Integer))
  (bind _asbp_third_person_character (Utilities|Casting|CastToBP_ThirdPersonCharacter OtherActor))
  (Variables|/Game/ThirdPerson/Blueprints/BP_ThirdPersonCharacter.BP_ThirdPersonCharacter_C|SetClosestButton _asbp_third_person_character 0))

(event Custom|ToggleButton
  (bind _output_get (Variables|Default|SetIsOn (not (Variables|Default|GetIsOn))))
  (Default|CallEDSwitch _output_get))

(fn ConstructionScript)