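; BP_SwitchButton is an interactable switch actor that lets the player turn a set of target objects on or off.
; When BP_ThirdPersonCharacter enters InteractionRadius, it creates a WBP_SwitchControl widget bound to itself and enables the mouse cursor with Game and UI input.
; Leaving the radius removes the widget and restores game-only input.
; Its Switchon and SwitchOff events relay SwitchOnMessage and SwitchOffMessage to every entry in TargetObjects.
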(event OnComponentEndOverlap(InteractionRadius)
  (params (OverlappedComponent :type Primitive%20Component%20Object%20Reference) (OtherActor :type Actor%20Object%20Reference) (OtherComp :type Primitive%20Component%20Object%20Reference) (OtherBodyIndex :type Integer))
  (bind _returnvalue (Game|GetPlayerController 0))
  (Utilities|Casting|CastToBP_ThirdPersonCharacter OtherActor)
  (Widget|RemovefromParent (Variables|Default|GetSwitchWidget))
  (Variables|Default|SetSwitchWidget 0)
  (Variables|/Script/Engine.PlayerController|SetbShowMouseCursor _returnvalue false)
  (Input|SetInputModeGameOnly _returnvalue false))

(event OnComponentBeginOverlap(InteractionRadius)
  (params (OverlappedComponent :type Primitive%20Component%20Object%20Reference) (OtherActor :type Actor%20Object%20Reference) (OtherComp :type Primitive%20Component%20Object%20Reference) (OtherBodyIndex :type Integer) (bFromSweep :type Boolean) (SweepResult :type Hit%20Result%20Structure%20%28by%20ref%29))
  (bind _returnvalue (Game|GetPlayerController 0))
  (Utilities|Casting|CastToBP_ThirdPersonCharacter OtherActor)
  (Utilities|IsValid (Variables|Default|GetSwitchWidget)
    (:Is%20Not%20Valid
      (bind _returnvalue_2 (UserInterface|CreateWidget "/Game/UMGSwtichable/Core/UI/WBP_SwitchControl.WBP_SwitchControl_C" 0 self))
      (bind _output_get (Variables|Default|SetSwitchWidget _returnvalue_2))
      (UserInterface|Viewport|AddtoViewport _output_get 0)
      (bind _output_get_2 (Variables|/Script/Engine.PlayerController|SetbShowMouseCursor _returnvalue true))
      (Input|SetInputModeGameandUI _returnvalue 0 "DoNotLock" _output_get_2 false))))

(event EventBeginPlay)

(event Collision|EventActorBeginOverlap
  (params (OtherActor :type Actor%20Object%20Reference)))

(event EventTick
  (params (DeltaSeconds :type Float%20%28single-precision%29)))

(event EventSwitchon
  (for _array_element (Variables|Default|GetTargetObjects)
    (Class|BPISwitchable|Switchon(Message) _array_element)))

(event EventSwitchOff
  (for _array_element (Variables|Default|GetTargetObjects)
    (Class|BPISwitchable|SwitchOff(Message) _array_element)))

(fn ConstructionScript)